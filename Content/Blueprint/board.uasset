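; Chess board actor that builds an 8x8 checkered board with pieces and handles click-to-move.
; The construction script spawns field and piece mesh components per square, choosing piece meshes from the Pos array and piece material by index.
; Click highlights the first chosen field, then moves that piece to the second, destroying any occupant without rule checks.
; Helper functions convert between square indices and positions on a fixed-spacing grid.
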(event EventBeginPlay)

(event Collision|EventActorBeginOverlap
  (params (OtherActor :type Actor%20Object%20Reference)))

(event EventTick
  (params (DeltaSeconds :type Float%20%28single-precision%29)))

(fn ConstructionScript
  (for _index (range 0 63)
    (Utilities|FlowControl|Sequence
      (:then_0
        (bind _returnvalue (AddComponent|AddStaticMeshComponent false (Math|Transform|MakeTransform (Utilities|Index->pos _index) "0, 0, 0" "10.000000,10.000000,10.000000")))
        (Utilities|Array|Add (Variables|Default|GetFieldsMesh) _returnvalue)
        (Rendering|Material|SetMaterial _returnvalue 0 (select (Class|KismetMathLibrary|XORBoolean (Math|Conversions|ToBoolean(Integer) (Math|Integer|%(Integer) _index 2)) (Math|Conversions|ToBoolean(Integer) (Math|Integer|%(Integer) (/ _index 8) 2))) "/Engine/MapTemplates/Materials/BasicTemplateMaterial.BasicTemplateMaterial" "/DatasmithContent/Materials/C4DMaster.C4DMaster"))
        (Utilities|Array|Add (Variables|Default|GetFieldsMaterial) (select (Class|KismetMathLibrary|XORBoolean (Math|Conversions|ToBoolean(Integer) (Math|Integer|%(Integer) _index 2)) (Math|Conversions|ToBoolean(Integer) (Math|Integer|%(Integer) (/ _index 8) 2))) "/Engine/MapTemplates/Materials/BasicTemplateMaterial.BasicTemplateMaterial" "/DatasmithContent/Materials/C4DMaster.C4DMaster")))
      (:then_1
        (bind _returnvalue_2 (AddComponent|AddStaticMeshComponent false (Math|Transform|MakeTransform (Utilities|Index->figurePos _index) "0,90.000000, 0" "10.000000,10.000000,10.000000")))
        (Components|StaticMesh|SetStaticMesh _returnvalue_2 (Utilities|Select :Index (Utilities|Array|Get(acopy) (Variables|Default|Getpos) _index) :Option%200 0 :Option%201 "/Game/Asset/CPawn_body1.CPawn_body1" :Option%202 "/Game/Asset/CRook_body1.CRook_body1" :Option%203 "/Game/Asset/CKnight_body1.CKnight_body1" :Option%204 "/Game/Asset/CBishop_body1.CBishop_body1" :Option%205 "/Game/Asset/CQueen_body1.CQueen_body1" :Option%206 "/Game/Asset/CKing_body1.CKing_body1"))
        (Rendering|Material|SetMaterial _returnvalue_2 0 (select (> _index 32) "/Engine/VREditor/Devices/Vive/ViveControllerMaterial.ViveControllerMaterial" "/Engine/MapTemplates/Materials/BasicTemplateMaterial.BasicTemplateMaterial"))
        (Utilities|Array|Add (Variables|Default|Getpieces_Mesh) _returnvalue_2)))))

(fn Click
  (params (Pos :type Vector))
  (bind _returnvalue (Utilities|Pos->index Pos))
  (bind _fieldsmesh (Variables|Default|GetFieldsMesh))
  (bind _pieces_mesh (Variables|Default|Getpieces_Mesh))
  (if (== (Variables|Default|Getlast_click) -1)
    (Rendering|Material|SetMaterial (Utilities|Array|Get(acopy) _fieldsmesh _returnvalue) 0 "/DatasmithContent/Materials/AliasMaster.AliasMaster")
    (Variables|Default|Setlast_click _returnvalue)
    (else
      (Rendering|Material|SetMaterial (Utilities|Array|Get(acopy) _fieldsmesh (Variables|Default|Getlast_click)) 0 (Utilities|Array|Get(acopy) (Variables|Default|GetFieldsMaterial) (Variables|Default|Getlast_click)))
      (Components|DestroyComponent (Utilities|Array|Get(acopy) (Variables|Default|Getpieces_Mesh) _returnvalue))
      (Transformation|SetWorldLocation (Utilities|Array|Get(acopy) (Variables|Default|Getpieces_Mesh) (Variables|Default|Getlast_click)) (Utilities|Index->figurePos _returnvalue) false false)
      (Utilities|Array|SetArrayElem _pieces_mesh _returnvalue (Utilities|Array|Get(acopy) (Variables|Default|Getpieces_Mesh) (Variables|Default|Getlast_click)))
      (Utilities|Array|SetArrayElem _pieces_mesh (Variables|Default|Getlast_click) 0)
      (Variables|Default|Setlast_click -1))))