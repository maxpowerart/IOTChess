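; Chess board actor that spawns 64 checkered squares and the piece meshes in its construction script and runs turn-based, click-driven play.
; Click selects a piece, DisplayAvailableMoves and SetAsAvailableMove highlight its moves and captures, and a second click rebuilds the piece on the target square.
; Piece type and side are read from meshes and materials.
; Check detection is unfinished: never called, white king only, with disconnected diagonal, pawn and knight scans.
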(event EventBeginPlay)

(event Collision|EventActorBeginOverlap
  (params (OtherActor :type Actor%20Object%20Reference)))

(event EventTick
  (params (DeltaSeconds :type Float%20%28single-precision%29)))

(fn ConstructionScript
  (for _index (range 0 63)
    (Utilities|FlowControl|Sequence
      (:then_0
        (bind _returnvalue (AddComponent|AddStaticMeshComponent false (Math|Transform|MakeTransform (Utilities|Index->pos _index) "0, 0, 0" "10.000000,10.000000,10.000000")))
        (Utilities|Array|Add (Variables|Default|GetFieldsMesh) _returnvalue)
        (Rendering|Material|SetMaterial _returnvalue 0 (select (Class|KismetMathLibrary|XORBoolean (Math|Conversions|ToBoolean(Integer) (Math|Integer|%(Integer) _index 2)) (Math|Conversions|ToBoolean(Integer) (Math|Integer|%(Integer) (/ _index 8) 2))) "/Engine/MapTemplates/Materials/BasicTemplateMaterial.BasicTemplateMaterial" "/DatasmithContent/Materials/C4DMaster.C4DMaster"))
        (Utilities|Array|Add (Variables|Default|GetFieldsMaterial) (select (Class|KismetMathLibrary|XORBoolean (Math|Conversions|ToBoolean(Integer) (Math|Integer|%(Integer) _index 2)) (Math|Conversions|ToBoolean(Integer) (Math|Integer|%(Integer) (/ _index 8) 2))) "/Engine/MapTemplates/Materials/BasicTemplateMaterial.BasicTemplateMaterial" "/DatasmithContent/Materials/C4DMaster.C4DMaster")))
      (:then_1
        (Utilities|FigureCreating (Math|Transform|MakeTransform (Utilities|Index->figurePos _index) "0,90.000000, 0" "10.000000,10.000000,10.000000") (Utilities|Select :Index (Utilities|Array|Get(acopy) (Variables|Default|Getpos) _index) :Option%200 0 :Option%201 "/Game/Asset/CPawn_body1.CPawn_body1" :Option%202 "/Game/Asset/CRook_body1.CRook_body1" :Option%203 "/Game/Asset/CKnight_body1.CKnight_body1" :Option%204 "/Game/Asset/CBishop_body1.CBishop_body1" :Option%205 "/Game/Asset/CQueen_body1.CQueen_body1" :Option%206 "/Game/Asset/CKing_body1.CKing_body1") _index (select (> _index 47) "/DatasmithContent/Materials/C4DMaster.C4DMaster" (select (< _index 16) "/Engine/MapTemplates/Materials/BasicTemplateMaterial.BasicTemplateMaterial" 0)) (select (> _index 47) "/DatasmithContent/Materials/C4DMaster.C4DMaster" (select (< _index 16) "/Engine/MapTemplates/Materials/BasicTemplateMaterial.BasicTemplateMaterial" 0)))))))

(fn Click
  (params (Pos :type Vector))
  (bind _returnvalue (Utilities|Pos->index Pos))
  (bind _pieces_mesh (Variables|Default|Getpieces_Mesh))
  (bind _output (Utilities|Array|Get(acopy) _pieces_mesh _returnvalue))
  (bind _returnvalue_2 (Rendering|Material|GetMaterial _output _returnvalue))
  (if (== (Variables|Default|Getlast_click) -1) ; первое или второе нажатие
    (if (!= (Variables|/Script/Engine.StaticMeshComponent|GetStaticMesh (Utilities|Array|Get(acopy) (Variables|Default|Getpieces_Mesh) _returnvalue)) 0) ; существует ли фигура
      (if (Variables|Default|GetwhuteTurn) ; ход белых?
        (if (== _returnvalue_2 (Variables|Default|Getwhite)) ; правильно ли нажали
          (Rendering|Material|SetMaterial (Utilities|Array|Get(acopy) (Variables|Default|GetFieldsMesh) _returnvalue) 0 "/DatasmithContent/Materials/CE_OpaqueMaster.CE_OpaqueMaster" :!label _label)
          (Variables|Default|Setlast_click _returnvalue)
          (CallFunction|DisplayAvailableMoves))
        (elif (== _returnvalue_2 (Variables|Default|Getblack))
          (goto _label))))
    (else
      (bind _isavailableformove (CallFunction|IsAvailableforMove _returnvalue))
      (if (or (not _isavailableformove) (== (Variables|Default|Getlast_click) _returnvalue)) ; Нажатие туда же/ за пределы допустимых ходов
        (Variables|Default|Setlast_click -1)
        (CallFunction|RestoreField)
        (else
          (Rendering|Material|SetMaterial (Utilities|Array|Get(acopy) (Variables|Default|Getpieces_Mesh) (Variables|Default|Getlast_click)) 0 (Utilities|Array|Get(acopy) (Variables|Default|GetFieldsMaterial) (Variables|Default|Getlast_click)))
          (if (!= (Variables|/Script/Engine.StaticMeshComponent|GetStaticMesh (Utilities|Array|Get(acopy) (Variables|Default|Getpieces_Mesh) (Variables|Default|Getlast_click))) 0)
            (Components|DestroyComponent (Utilities|Array|Get(acopy) (Variables|Default|Getpieces_Mesh) _returnvalue))
            (bind _new_mesh (Utilities|FigureCreating (Math|Transform|MakeTransform (Utilities|Index->figurePos _returnvalue) "0,90.000000, 0" "10.000000,10.000000,10.000000") (Variables|/Script/Engine.StaticMeshComponent|GetStaticMesh (Utilities|Array|Get(acopy) (Variables|Default|Getpieces_Mesh) (Variables|Default|Getlast_click))) _returnvalue (select (Variables|Default|GetwhuteTurn) (Variables|Default|Getwhite) (Variables|Default|Getblack)) (select (Variables|Default|GetwhuteTurn) (Variables|Default|Getwhite) (Variables|Default|Getblack)))
              (:%20
                (Components|DestroyComponent (Utilities|Array|Get(acopy) (Variables|Default|Getpieces_Mesh) (Variables|Default|Getlast_click)))
                (Utilities|Array|SetArrayElem (Variables|Default|Getpieces_Mesh) _returnvalue _new_mesh)
                (Rendering|Material|SetMaterial (Utilities|Array|Get(acopy) (Variables|Default|Getpieces_Mesh) (Variables|Default|Getlast_click)) _returnvalue (select (Variables|Default|GetwhuteTurn) (Variables|Default|Getwhite) (Variables|Default|Getblack)))
                (Variables|Default|Setlast_click -1)
                (Variables|Default|SetwhuteTurn (not (Variables|Default|GetwhuteTurn)))
                (CallFunction|RestoreField)))))))))

(fn DisplayAvailableMoves
  (bind _pieces_mesh (Variables|Default|Getpieces_Mesh))
  (bind _last_click (Variables|Default|Getlast_click))
  (bind _last_click_2 (Variables|Default|Getlast_click))
  (bind _last_click_3 (Variables|Default|Getlast_click))
  (bind _output (Utilities|Array|Get(acopy) _pieces_mesh _last_click))
  (bind _staticmesh (Variables|/Script/Engine.StaticMeshComponent|GetStaticMesh _output))
  (Utilities|Array|Clear (Variables|Default|GetAvailableMoves))
  (if (== _staticmesh "/Game/Asset/CKing_body1.CKing_body1")
    ;[1 1 1] King
    (for _index (range -1 1)
      (for _index_2 (range -1 1)
        (if (!= (+ (* _index 8) _index_2 _last_click_2) _last_click_2)
          (CallFunction|SetasAvailableMove (+ (* _index 8) _index_2 _last_click_2) true true false))))
    (elif (== _staticmesh "/Game/Asset/CQueen_body1.CQueen_body1")
      ;[1 1 1] Queen
      (bind _array_element (Utilities|Array|ForEachLoopwithBreak (Utilities|Array|MakeArray -9 -8 -7 -1 1 7 8 9))
        (:LoopBody
          (bind _index_3 (Utilities|FlowControl|ForLoopwithBreak 1 7 :!label _label)
            (:LoopBody
              (bind _successful (CallFunction|SetasAvailableMove (+ (* _index_3 _array_element) (Variables|Default|Getlast_click)) true false false))
              (if (not _successful)
                (goto _label Break))))))
      (elif (== _staticmesh "/Game/Asset/CBishop_body1.CBishop_body1")
        ;[1 1 1] Bishop
        (bind _array_element_2 (Utilities|Array|ForEachLoopwithBreak (Utilities|Array|MakeArray -9 -7 7 9))
          (:LoopBody
            (bind _index_4 (Utilities|FlowControl|ForLoopwithBreak 1 7 :!label _label_2)
              (:LoopBody
                (bind _successful_2 (CallFunction|SetasAvailableMove (+ (* _index_4 _array_element_2) (Variables|Default|Getlast_click)) true false false))
                (if (not _successful_2)
                  (goto _label_2 Break))))))
        (elif (== _staticmesh "/Game/Asset/CRook_body1.CRook_body1")
          ;[1 1 1] Rook
          (bind _array_element_3 (Utilities|Array|ForEachLoopwithBreak (Utilities|Array|MakeArray -8 -1 1 8))
            (:LoopBody
              (bind _index_5 (Utilities|FlowControl|ForLoopwithBreak 1 7 :!label _label_3)
                (:LoopBody
                  (bind _successful_3 (CallFunction|SetasAvailableMove (+ (* _index_5 _array_element_3) (Variables|Default|Getlast_click)) true false false))
                  (if (not _successful_3)
                    (goto _label_3 Break))))))
          (elif (== _staticmesh "/Game/Asset/CKnight_body1.CKnight_body1")
            ;[1 1 1] Knight
            (for _array_element_4 (Utilities|Array|MakeArray -17 -15 -10 -6 6 10 15 17)
              (CallFunction|SetasAvailableMove (+ _array_element_4 (Variables|Default|Getlast_click)) true true false))
            (elif (== _staticmesh "/Game/Asset/CPawn_body1.CPawn_body1")
              ;[1 1 1] Pawn
              (for (_array_element_5 _array_index) (Utilities|Array|MakeArray 7 9 8 16)
                (if (< _array_index 3)
                  (CallFunction|SetasAvailableMove (+ _last_click_3 (* _array_element_5 (+ (* (Math|Conversions|ToInteger(Boolean) (Variables|Default|GetwhuteTurn)) 2) -1))) false true (or (== _array_element_5 7) (== _array_element_5 9)) :!label _label_4)
                  (elif (Utilities|CanMakeDoubleMove _last_click_3)
                    (goto _label_4)))))))))))

(fn SetasAvailableMove
  (params (Ind :type Integer) (CnBite :type Boolean) (No%20Trace :type Boolean) (Pawn%20Side%20Bite :type Boolean))
  (bind _isenemy (CallFunction|IsEnemy Ind))
  (if (Math|Boolean|ANDBoolean (< Ind 64) (> Ind -1) (and No%20Trace (< (Math|Vector|VectorLength (- (Utilities|Index->pos (Variables|Default|Getlast_click)) (Utilities|Index->pos Ind))) 2.5e+02)))
    (bind _clear (CallFunction|IsCeilClear Ind))
    (if (or (Class|KismetMathLibrary|XORBoolean _clear Pawn%20Side%20Bite) (and (or Pawn%20Side%20Bite CnBite) _isenemy))
      (Rendering|Material|SetMaterial (Utilities|Array|Get(acopy) (Variables|Default|GetFieldsMesh) Ind) 0 (select (and (or Pawn%20Side%20Bite CnBite) _isenemy) "/AnimationSharing/AnimSharingRed.AnimSharingRed" "/AnimationSharing/AnimSharingGreen.AnimSharingGreen"))
      (Utilities|Array|Add (Variables|Default|GetAvailableMoves) Ind)
      (return (and (and (!= (Math|Integer|%(Integer) Ind 8) 0) (!= (Math|Integer|%(Integer) (+ Ind 1) 8) 0)) (not (and (or Pawn%20Side%20Bite CnBite) _isenemy))))
      (else
        _)))
  (return false))

(fn IsEnemy
  (params (indx :type Integer))
  (bind _pieces_mesh (Variables|Default|Getpieces_Mesh))
  (bind _output (Utilities|Array|Get(acopy) _pieces_mesh indx))
  (bind _returnvalue (Rendering|Material|GetMaterial _output 0))
  (if (== _returnvalue 0)
    (return false)
    (else
      (return (!= _returnvalue (Rendering|Material|GetMaterial (Utilities|Array|Get(acopy) (Variables|Default|Getpieces_Mesh) (Variables|Default|Getlast_click)) 0))))))

(fn IsCeilClear
  (params (Index :type Integer))
  (return (== (Variables|/Script/Engine.StaticMeshComponent|GetStaticMesh (Utilities|Array|Get(acopy) (Variables|Default|Getpieces_Mesh) Index)) 0)))

(fn RestoreField
  (for (_array_element _array_index) (Variables|Default|GetFieldsMesh)
    (Rendering|Material|SetMaterial _array_element 0 (Utilities|Array|Get(acopy) (Variables|Default|GetFieldsMaterial) _array_index))
    (if (== (Variables|/Script/Engine.StaticMeshComponent|GetStaticMesh (Utilities|Array|Get(acopy) (Variables|Default|Getpieces_Mesh) _array_index)) "/Game/Asset/CKing_body1.CKing_body1")
      (if (== (Rendering|Material|GetMaterial (Utilities|Array|Get(acopy) (Variables|Default|Getpieces_Mesh) _array_index) _array_index) (Variables|Default|Getwhite))
        (Variables|Default|SetWhiteKing _array_index)
        (else
          (Variables|Default|SetBlackKing _array_index))))))

(fn IsAvailableforMove
  (params (index :type Integer))
  (return (!= (Utilities|Array|FindItem (Variables|Default|GetAvailableMoves) index) -1)))

(fn Check
  (params (White :type Boolean))
  (if White
    ;[1 1 1] Проверка на прямые (ладья/ферзь)
    (LocalVariables|Setscouter (+ (Variables|Default|GetWhiteKing) 8))
    (while (Math|Boolean|ANDBoolean (< (LocalVariables|Getscouter) 0) (> (LocalVariables|Getscouter) 63) (!= (Rendering|Material|GetMaterial (Utilities|Array|Get(acopy) (Variables|Default|GetFieldsMesh) (LocalVariables|Getscouter)) (LocalVariables|Getscouter)) (Variables|Default|Getwhite)) (not (and (or (== (Utilities|Array|Get(acopy) (Variables|Default|GetFieldsMesh) (LocalVariables|Getscouter)) "/Game/Asset/CRook_body1.CRook_body1") (== (Utilities|Array|Get(acopy) (Variables|Default|GetFieldsMesh) (LocalVariables|Getscouter)) "/Game/Asset/CQueen_body1.CQueen_body1")) (== (Rendering|Material|GetMaterial (Utilities|Array|Get(acopy) (Variables|Default|GetFieldsMesh) (LocalVariables|Getscouter)) (LocalVariables|Getscouter)) (Variables|Default|Getblack))))) ; Проверка вверх
      (LocalVariables|Setscouter (+ (LocalVariables|Getscouter) 8))
      (if (and (or (== (Utilities|Array|Get(acopy) (Variables|Default|GetFieldsMesh) (LocalVariables|Getscouter)) "/Game/Asset/CRook_body1.CRook_body1") (== (Utilities|Array|Get(acopy) (Variables|Default|GetFieldsMesh) (LocalVariables|Getscouter)) "/Game/Asset/CQueen_body1.CQueen_body1")) (== (Rendering|Material|GetMaterial (Utilities|Array|Get(acopy) (Variables|Default|GetFieldsMesh) (LocalVariables|Getscouter)) (LocalVariables|Getscouter)) (Variables|Default|Getblack)))
        (LocalVariables|Setshah (and (or (== (Utilities|Array|Get(acopy) (Variables|Default|GetFieldsMesh) (LocalVariables|Getscouter)) "/Game/Asset/CRook_body1.CRook_body1") (== (Utilities|Array|Get(acopy) (Variables|Default|GetFieldsMesh) (LocalVariables|Getscouter)) "/Game/Asset/CQueen_body1.CQueen_body1")) (== (Rendering|Material|GetMaterial (Utilities|Array|Get(acopy) (Variables|Default|GetFieldsMesh) (LocalVariables|Getscouter)) (LocalVariables|Getscouter)) (Variables|Default|Getblack))))))
    (if (> (LocalVariables|Getscouter) 63)
      (LocalVariables|Setscouter (- (Variables|Default|GetWhiteKing) 8))
      (while (Math|Boolean|ANDBoolean (< (LocalVariables|Getscouter) 0) (> (LocalVariables|Getscouter) 63) (!= (Rendering|Material|GetMaterial (Utilities|Array|Get(acopy) (Variables|Default|GetFieldsMesh) (LocalVariables|Getscouter)) (LocalVariables|Getscouter)) (Variables|Default|Getwhite)) (not (and (or (== (Utilities|Array|Get(acopy) (Variables|Default|GetFieldsMesh) (LocalVariables|Getscouter)) "/Game/Asset/CRook_body1.CRook_body1") (== (Utilities|Array|Get(acopy) (Variables|Default|GetFieldsMesh) (LocalVariables|Getscouter)) "/Game/Asset/CQueen_body1.CQueen_body1")) (== (Rendering|Material|GetMaterial (Utilities|Array|Get(acopy) (Variables|Default|GetFieldsMesh) (LocalVariables|Getscouter)) (LocalVariables|Getscouter)) (Variables|Default|Getblack))))) ; Проверка вниз
        (LocalVariables|Setscouter (- (LocalVariables|Getscouter) 8))
        (if (and (or (== (Utilities|Array|Get(acopy) (Variables|Default|GetFieldsMesh) (LocalVariables|Getscouter)) "/Game/Asset/CRook_body1.CRook_body1") (== (Utilities|Array|Get(acopy) (Variables|Default|GetFieldsMesh) (LocalVariables|Getscouter)) "/Game/Asset/CQueen_body1.CQueen_body1")) (== (Rendering|Material|GetMaterial (Utilities|Array|Get(acopy) (Variables|Default|GetFieldsMesh) (LocalVariables|Getscouter)) (LocalVariables|Getscouter)) (Variables|Default|Getblack)))
          (LocalVariables|Setshah (and (or (== (Utilities|Array|Get(acopy) (Variables|Default|GetFieldsMesh) (LocalVariables|Getscouter)) "/Game/Asset/CRook_body1.CRook_body1") (== (Utilities|Array|Get(acopy) (Variables|Default|GetFieldsMesh) (LocalVariables|Getscouter)) "/Game/Asset/CQueen_body1.CQueen_body1")) (== (Rendering|Material|GetMaterial (Utilities|Array|Get(acopy) (Variables|Default|GetFieldsMesh) (LocalVariables|Getscouter)) (LocalVariables|Getscouter)) (Variables|Default|Getblack))))))
      (if (< (LocalVariables|Getscouter) 0)
        (LocalVariables|Setscouter (- (Variables|Default|GetWhiteKing) 1))
        (while (and (Math|Boolean|ANDBoolean (< (LocalVariables|Getscouter) 0) (> (LocalVariables|Getscouter) 63) (!= (Rendering|Material|GetMaterial (Utilities|Array|Get(acopy) (Variables|Default|GetFieldsMesh) (LocalVariables|Getscouter)) (LocalVariables|Getscouter)) (Variables|Default|Getwhite)) (not (and (or (== (Utilities|Array|Get(acopy) (Variables|Default|GetFieldsMesh) (LocalVariables|Getscouter)) "/Game/Asset/CRook_body1.CRook_body1") (== (Utilities|Array|Get(acopy) (Variables|Default|GetFieldsMesh) (LocalVariables|Getscouter)) "/Game/Asset/CQueen_body1.CQueen_body1")) (== (Rendering|Material|GetMaterial (Utilities|Array|Get(acopy) (Variables|Default|GetFieldsMesh) (LocalVariables|Getscouter)) (LocalVariables|Getscouter)) (Variables|Default|Getblack))))) (not (Utilities|TooFarLeft (LocalVariables|Getscouter)))) ; Проверка влево
          (LocalVariables|Setscouter (- (LocalVariables|Getscouter) 1))
          (if (and (or (== (Utilities|Array|Get(acopy) (Variables|Default|GetFieldsMesh) (LocalVariables|Getscouter)) "/Game/Asset/CRook_body1.CRook_body1") (== (Utilities|Array|Get(acopy) (Variables|Default|GetFieldsMesh) (LocalVariables|Getscouter)) "/Game/Asset/CQueen_body1.CQueen_body1")) (== (Rendering|Material|GetMaterial (Utilities|Array|Get(acopy) (Variables|Default|GetFieldsMesh) (LocalVariables|Getscouter)) (LocalVariables|Getscouter)) (Variables|Default|Getblack)))
            (LocalVariables|Setshah (and (or (== (Utilities|Array|Get(acopy) (Variables|Default|GetFieldsMesh) (LocalVariables|Getscouter)) "/Game/Asset/CRook_body1.CRook_body1") (== (Utilities|Array|Get(acopy) (Variables|Default|GetFieldsMesh) (LocalVariables|Getscouter)) "/Game/Asset/CQueen_body1.CQueen_body1")) (== (Rendering|Material|GetMaterial (Utilities|Array|Get(acopy) (Variables|Default|GetFieldsMesh) (LocalVariables|Getscouter)) (LocalVariables|Getscouter)) (Variables|Default|Getblack))))))
        (if (Utilities|TooFarLeft (LocalVariables|Getscouter))
          (LocalVariables|Setscouter (+ (Variables|Default|GetWhiteKing) 1))
          (while (and (Math|Boolean|ANDBoolean (< (LocalVariables|Getscouter) 0) (> (LocalVariables|Getscouter) 63) (!= (Rendering|Material|GetMaterial (Utilities|Array|Get(acopy) (Variables|Default|GetFieldsMesh) (LocalVariables|Getscouter)) (LocalVariables|Getscouter)) (Variables|Default|Getwhite)) (not (and (or (== (Utilities|Array|Get(acopy) (Variables|Default|GetFieldsMesh) (LocalVariables|Getscouter)) "/Game/Asset/CRook_body1.CRook_body1") (== (Utilities|Array|Get(acopy) (Variables|Default|GetFieldsMesh) (LocalVariables|Getscouter)) "/Game/Asset/CQueen_body1.CQueen_body1")) (== (Rendering|Material|GetMaterial (Utilities|Array|Get(acopy) (Variables|Default|GetFieldsMesh) (LocalVariables|Getscouter)) (LocalVariables|Getscouter)) (Variables|Default|Getblack))))) (not (Utilities|TooFarRight (LocalVariables|Getscouter)))) ; Проверка вправо
            (LocalVariables|Setscouter (+ (LocalVariables|Getscouter) 1))
            (if (and (or (== (Utilities|Array|Get(acopy) (Variables|Default|GetFieldsMesh) (LocalVariables|Getscouter)) "/Game/Asset/CRook_body1.CRook_body1") (== (Utilities|Array|Get(acopy) (Variables|Default|GetFieldsMesh) (LocalVariables|Getscouter)) "/Game/Asset/CQueen_body1.CQueen_body1")) (== (Rendering|Material|GetMaterial (Utilities|Array|Get(acopy) (Variables|Default|GetFieldsMesh) (LocalVariables|Getscouter)) (LocalVariables|Getscouter)) (Variables|Default|Getblack)))
              (LocalVariables|Setshah (and (or (== (Utilities|Array|Get(acopy) (Variables|Default|GetFieldsMesh) (LocalVariables|Getscouter)) "/Game/Asset/CRook_body1.CRook_body1") (== (Utilities|Array|Get(acopy) (Variables|Default|GetFieldsMesh) (LocalVariables|Getscouter)) "/Game/Asset/CQueen_body1.CQueen_body1")) (== (Rendering|Material|GetMaterial (Utilities|Array|Get(acopy) (Variables|Default|GetFieldsMesh) (LocalVariables|Getscouter)) (LocalVariables|Getscouter)) (Variables|Default|Getblack))))))
          (if (Utilities|TooFarRight (LocalVariables|Getscouter))
            (LocalVariables|Setscouter (Variables|Default|GetWhiteKing))))))))